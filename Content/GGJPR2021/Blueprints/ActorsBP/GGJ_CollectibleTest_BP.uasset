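; Test collectible Blueprint: a spinning coin that destroys itself with an explosion effect and sound on box overlap.
; Tick rotates the coin around yaw, scaled by delta time, and the box trigger responds to any overlapping actor.
; A separate sphere trigger reacts only to the first-person character, showing a widget and setting a placeholder boolean while overlapped, then reversing both on exit.
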(event `self.Box.OnComponentBeginOverlap`
  (params (OverlappedComponent :type "PrimitiveComponent Object Reference") (OtherActor :type "Actor Object Reference") (OtherComp :type "PrimitiveComponent Object Reference") (OtherBodyIndex :type Integer) (bFromSweep :type Boolean) (SweepResult :type "HitResult Structure (by ref)"))
  (bind _returnvalue (`self.K2_GetActorLocation`))
  (`self.K2_DestroyActor`)
  (`GameplayStatics.SpawnEmitterAtLocation` "/Game/StarterContent/Particles/P_Explosion.P_Explosion" _returnvalue)
  (`GameplayStatics.PlaySoundAtLocation` "/Game/StarterContent/Audio/Explosion_Cue.Explosion_Cue" _returnvalue (struct) 1.0 1.0 0.0 null null null))

(event `self.ReceiveTick`
  (params (DeltaSeconds :type "Float (single-precision)"))
  (`SceneComponent.K2_AddLocalRotation` (`self.Coin`) (* (`KismetMathLibrary.MakeRotator` 0.0 0.0 150.0) DeltaSeconds) false false))

(event `self.Sphere.OnComponentBeginOverlap`
  (params (OverlappedComponent :type "PrimitiveComponent Object Reference") (OtherActor :type "Actor Object Reference") (OtherComp :type "PrimitiveComponent Object Reference") (OtherBodyIndex :type Integer) (bFromSweep :type Boolean) (SweepResult :type "HitResult Structure (by ref)"))
  (cast `/Game/GGJPR2021/Blueprints/FirstPersonBP/GGJ_FirstPersonCharacter_BP` OtherActor)
  (`SceneComponent.SetVisibility` (`self.Widget`) true false)
  (set `self.TestBoolean` true) ; In case you need a specific function to work with this boolean
)

(event `self.Sphere.OnComponentEndOverlap`
  (params (OverlappedComponent :type "PrimitiveComponent Object Reference") (OtherActor :type "Actor Object Reference") (OtherComp :type "PrimitiveComponent Object Reference") (OtherBodyIndex :type Integer))
  (cast `/Game/GGJPR2021/Blueprints/FirstPersonBP/GGJ_FirstPersonCharacter_BP` OtherActor)
  (`SceneComponent.SetVisibility` (`self.Widget`) false false)
  (set `self.TestBoolean` false))

(fn `UserConstructionScript`)