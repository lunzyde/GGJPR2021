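; Level goal trigger that advances or ends the game when the first-person character or tractor overlaps its box.
; If NextLevel names the Plains level, it opens that level.
; Any other value shows the GGJArt image on the game mode's main widget, disables player input and shows the mouse cursor, apparently as an end screen.
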(event `self.Box.OnComponentBeginOverlap`
  (params (OverlappedComponent :type "PrimitiveComponent Object Reference") (OtherActor :type "Actor Object Reference") (OtherComp :type "PrimitiveComponent Object Reference") (OtherBodyIndex :type Integer) (bFromSweep :type Boolean) (SweepResult :type "HitResult Structure (by ref)"))
  (bind _returnvalue (`GameplayStatics.GetPlayerController` 0))
  (bind _nextlevel (`self.NextLevel`))
  (cast `/Game/GGJPR2021/Blueprints/FirstPersonBP/GGJ_FirstPersonCharacter_BP` OtherActor
    (:`then`
      _)
    (:`CastFailed`
      (cast `/Game/GGJPR2021/Blueprints/TractorBP/GGJ_TractorBP` OtherActor)))
  (switch `name` _nextlevel
    (:`Default`
      (bind _asggj_first_person_game_mode (cast `/Game/GGJPR2021/Blueprints/GameModesBP/GGJ_FirstPerson_GameMode` (`GameplayStatics.GetGameMode`)))
      (`Widget.SetVisibility` (`/Game/GGJPR2021/Blueprints/UserInterfaceBP/GGJ_Main_WB.GGJ_Art` (`/Game/GGJPR2021/Blueprints/GameModesBP/GGJ_FirstPerson_GameMode.MainWidget` _asggj_first_person_game_mode)) "Visible")
      (`self.DisableInput` _returnvalue _returnvalue)
      (set `PlayerController.bShowMouseCursor` true _returnvalue))
    (:`GGJ_ThePlains_Level`
      (`GameplayStatics.OpenLevel` _nextlevel))))

(fn `UserConstructionScript`)