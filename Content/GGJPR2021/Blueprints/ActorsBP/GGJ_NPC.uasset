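; GGJ_NPC is an NPC actor the first-person player can talk to when nearby.
; An interaction sphere toggles its prompt widget and interactable flag, and registers the NPC on the player character and the player on its interactable component.
; Each Interact call shows the next dialogue line in the game mode's main widget text box and flags the player as talking, hiding and resetting once lines run out.
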(event `self.ReceiveBeginPlay`
  (bind _asggj_first_person_game_mode (cast `/Game/GGJPR2021/Blueprints/GameModesBP/GGJ_FirstPerson_GameMode` (`GameplayStatics.GetGameMode`)))
  (set `self.TextBox` (`/Game/GGJPR2021/Blueprints/UserInterfaceBP/GGJ_Main_WB.GGJ_TextBox` (`/Game/GGJPR2021/Blueprints/GameModesBP/GGJ_FirstPerson_GameMode.MainWidget` _asggj_first_person_game_mode))))

(event `self.InteractionSphere.OnComponentBeginOverlap`
  (params (OverlappedComponent :type "PrimitiveComponent Object Reference") (OtherActor :type "Actor Object Reference") (OtherComp :type "PrimitiveComponent Object Reference") (OtherBodyIndex :type Integer) (bFromSweep :type Boolean) (SweepResult :type "HitResult Structure (by ref)"))
  (bind _asggj_first_person_character_bp (cast `/Game/GGJPR2021/Blueprints/FirstPersonBP/GGJ_FirstPersonCharacter_BP` OtherActor))
  (set `/Game/GGJPR2021/Blueprints/ActorsBP/GGJ_InteractableBP.PlayerCharacter` _asggj_first_person_character_bp (`self.GGJ_InteractableBP`))
  (set `self.Interactable?` true)
  (set `/Game/GGJPR2021/Blueprints/FirstPersonBP/GGJ_FirstPersonCharacter_BP.NPC` self _asggj_first_person_character_bp)
  (`SceneComponent.SetVisibility` (`self.Widget`) true false))

(event `self.InteractionSphere.OnComponentEndOverlap`
  (params (OverlappedComponent :type "PrimitiveComponent Object Reference") (OtherActor :type "Actor Object Reference") (OtherComp :type "PrimitiveComponent Object Reference") (OtherBodyIndex :type Integer))
  (bind _asggj_first_person_character_bp (cast `/Game/GGJPR2021/Blueprints/FirstPersonBP/GGJ_FirstPersonCharacter_BP` OtherActor))
  (set `/Game/GGJPR2021/Blueprints/ActorsBP/GGJ_InteractableBP.PlayerCharacter` null (`self.GGJ_InteractableBP`))
  (set `self.Interactable?` false)
  (set `/Game/GGJPR2021/Blueprints/FirstPersonBP/GGJ_FirstPersonCharacter_BP.NPC` null _asggj_first_person_character_bp)
  (`SceneComponent.SetVisibility` (`self.Widget`) false false))

(event `Interact`
  (bind _textbox (`self.TextBox`))
  (bind _textbox_2 (`self.TextBox`))
  (if (and (`self.Interactable?`) (< (`self.DialogueIndex`) (`KismetArrayLibrary.Array_Length` (`self.Dialogue`))))
    (`Widget.SetVisibility` _textbox "Visible")
    (`/Game/GGJPR2021/Blueprints/UserInterfaceBP/GGJ_TextBox.SetText` _textbox (`|GetArrayItem` (`self.Dialogue`) (`self.DialogueIndex`)))
    (`/Engine/EditorBlueprintResources/StandardMacros.IncrementInt` (`self.DialogueIndex`)
      (:`  `
        (set `/Game/GGJPR2021/Blueprints/FirstPersonBP/GGJ_FirstPersonCharacter_BP.Talking?` true (`/Game/GGJPR2021/Blueprints/ActorsBP/GGJ_InteractableBP.PlayerCharacter` (`self.GGJ_InteractableBP`)))))
    (else
      (`Widget.SetVisibility` _textbox_2 "Collapsed")
      (set `self.DialogueIndex` 0)
      (`/Game/GGJPR2021/Blueprints/UserInterfaceBP/GGJ_TextBox.SetText` _textbox_2 "")
      (set `/Game/GGJPR2021/Blueprints/FirstPersonBP/GGJ_FirstPersonCharacter_BP.Talking?` false (`/Game/GGJPR2021/Blueprints/ActorsBP/GGJ_InteractableBP.PlayerCharacter` (`self.GGJ_InteractableBP`))))))

(fn `UserConstructionScript`)