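; Drivable tractor pawn that the first-person character can interact with, flagged through a box overlap that also shows a widget.
; Each tick traces down from every wheel position, pushing the physics cube up by suspension compression, then applies throttle force and steering impulse that inverts in reverse.
; Input orbits the spring arm, while camera pitch and engine sound pitch ease with view and throttle.
; Exit repossesses the character nearby; Reset reloads the level.
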(event `InputAxis|Turn`
  (params (AxisValue :type "Float (single-precision)"))
  (bind _springarm (`self.SpringArm`))
  (bind (_relativerotation_roll _relativerotation_pitch _relativerotation_yaw) (`KismetMathLibrary.BreakRotator` (`SceneComponent.RelativeRotation` _springarm)))
  (`SceneComponent.K2_SetRelativeRotation` _springarm (`KismetMathLibrary.MakeRotator` _relativerotation_roll _relativerotation_pitch (`KismetMathLibrary.ClampAxis` (+ AxisValue _relativerotation_yaw))) false false))

(event `InputAxis|LookUp`
  (params (AxisValue :type "Float (single-precision)"))
  (bind _springarm (`self.SpringArm`))
  (bind (_relativerotation_roll _relativerotation_pitch _relativerotation_yaw) (`KismetMathLibrary.BreakRotator` (`SceneComponent.RelativeRotation` _springarm)))
  (`SceneComponent.K2_SetRelativeRotation` _springarm (`KismetMathLibrary.MakeRotator` _relativerotation_roll (`KismetMathLibrary.ClampAxis` (`KismetMathLibrary.ClampAngle` (- _relativerotation_pitch AxisValue) -55.0 15.0)) _relativerotation_yaw) false false))

(event `self.ReceiveBeginPlay`
  (bind _niagara (`self.Niagara`))
  (`/Game/GGJPR2021/Blueprints/ActorsBP/GGJ_Niagara.ActivateNiagra` (`self.GGJ_Niagara`) _niagara)
  (`ActorComponent.Deactivate` _niagara))

(event `InputAxis|MoveRight` :overrideparent false
  (params (AxisValue :type "Float (single-precision)"))
  (if (== (`GameplayStatics.GetPlayerPawn` 0) self)
    (set `self.Steer` AxisValue)))

(event `InputAxis|MoveForward` :overrideparent false
  (params (AxisValue :type "Float (single-precision)"))
  (bind _throttle (`self.Throttle`))
  (if (== (`GameplayStatics.GetPlayerPawn` 0) self)
    (if (== AxisValue 0.0)
      (set `self.Throttle` (`KismetMathLibrary.Abs` _throttle)))
    (set `self.Throttle` (`KismetMathLibrary.Lerp` _throttle AxisValue (`self.ThrottleSensitivity`)))))

(event `self.ReceiveTick`
  (params (DeltaSeconds :type "Float (single-precision)"))
  (bind _camera (`self.Camera`))
  (bind _enginesound (`self.EngineSound`))
  (bind (_returnvalue_roll _returnvalue_pitch) (`KismetMathLibrary.BreakRotator` (`SceneComponent.K2_GetComponentRotation` _camera)))
  (bind (_relativerotation_roll _relativerotation_pitch) (`KismetMathLibrary.BreakRotator` (`SceneComponent.RelativeRotation` (`self.SpringArm`))))
  (bind _pitchmultiplier (`AudioComponent.PitchMultiplier` _enginesound))
  (`self.CalcWheelHits`)
  (`self.ApplyImpulses`)
  (`SceneComponent.K2_AddLocalRotation` _camera (`KismetMathLibrary.MakeRotator` 0.0 (* DeltaSeconds (`KismetMathLibrary.Lerp` 0.0 (- (+ -2.0 (/ _relativerotation_pitch 0.9)) _returnvalue_pitch) 0.8))) false false)
  (`AudioComponent.SetPitchMultiplier` _enginesound (+ _pitchmultiplier (* DeltaSeconds (`KismetMathLibrary.Lerp` 0.0 (- (+ 1.0 (/ (`KismetMathLibrary.Abs` (`self.Throttle`)) 1.2)) _pitchmultiplier) 0.5)))))

(event `self.Box.OnComponentBeginOverlap`
  (params (OverlappedComponent :type "PrimitiveComponent Object Reference") (OtherActor :type "Actor Object Reference") (OtherComp :type "PrimitiveComponent Object Reference") (OtherBodyIndex :type Integer) (bFromSweep :type Boolean) (SweepResult :type "HitResult Structure (by ref)"))
  (bind _asggj_first_person_character_bp (cast `/Game/GGJPR2021/Blueprints/FirstPersonBP/GGJ_FirstPersonCharacter_BP` OtherActor))
  (bind _output_get (set `/Game/GGJPR2021/Blueprints/ActorsBP/GGJ_InteractableBP.PlayerCharacter` _asggj_first_person_character_bp (`self.GGJ_InteractableBP`)))
  (set `/Game/GGJPR2021/Blueprints/FirstPersonBP/GGJ_FirstPersonCharacter_BP.IsOverlapped?` true _output_get)
  (set `/Game/GGJPR2021/Blueprints/FirstPersonBP/GGJ_FirstPersonCharacter_BP.InteractableActor` self _output_get)
  (`SceneComponent.SetVisibility` (`self.Widget`) true false))

(event `self.Box.OnComponentEndOverlap`
  (params (OverlappedComponent :type "PrimitiveComponent Object Reference") (OtherActor :type "Actor Object Reference") (OtherComp :type "PrimitiveComponent Object Reference") (OtherBodyIndex :type Integer))
  (bind _asggj_first_person_character_bp (cast `/Game/GGJPR2021/Blueprints/FirstPersonBP/GGJ_FirstPersonCharacter_BP` OtherActor))
  (set `/Game/GGJPR2021/Blueprints/FirstPersonBP/GGJ_FirstPersonCharacter_BP.IsOverlapped?` false _asggj_first_person_character_bp)
  (set `/Game/GGJPR2021/Blueprints/FirstPersonBP/GGJ_FirstPersonCharacter_BP.InteractableActor` null _asggj_first_person_character_bp)
  (`SceneComponent.SetVisibility` (`self.Widget`) false false))

(event `InputAction|Reset`
  (params (Key :type "Key Structure"))
  (:`Pressed`
    (bind _returnvalue (`GameplayStatics.GetCurrentLevelName` true))
    (`GameplayStatics.OpenLevel` (`KismetStringLibrary.Conv_StringToName` _returnvalue))))

(event `Exit`
  (bind (_returnvalue_x _returnvalue_y _returnvalue_z) (`KismetMathLibrary.BreakVector` (`self.K2_GetActorLocation`)))
  (bind _playercharacter (`/Game/GGJPR2021/Blueprints/ActorsBP/GGJ_InteractableBP.PlayerCharacter` (`self.GGJ_InteractableBP`))
    (:`then`
      (`Controller.Possess` (`GameplayStatics.GetPlayerController` 0) _playercharacter)
      (`ActorComponent.Activate` (`/Game/GGJPR2021/Blueprints/FirstPersonBP/GGJ_FirstPersonCharacter_BP.NiagaraSystem` _playercharacter) false)
      (`ActorComponent.Deactivate` (`self.Niagara`))
      (set `self.Throttle` 0.0)
      (set `self.Steer` 0.0)
      (`self.K2_SetActorLocation` _playercharacter (`KismetMathLibrary.MakeVector` (+ _returnvalue_x 1000.0) (+ _returnvalue_y 1000.0) (+ _returnvalue_z 100.0)) false false))
    (:`else`)))

(event `self.ReceivePossessed`
  (params (NewController :type "Controller Object Reference"))
  (cast `PlayerController` NewController)
  (`ActorComponent.Activate` (`self.Niagara`) false))

(fn `ApplyImpulses`
  (bind _throttle (`self.Throttle`))
  (bind _cube (`self.Cube`))
  (bind _cube_2 (`self.Cube`))
  (bind _returnvalue (* 3.0 (`self.Steer`)))
  (bind (_returnvalue_x _returnvalue_y) (`KismetMathLibrary.BreakVector` (* (1.0 0.0 0.0) (* (`PrimitiveComponent.GetMass` _cube_2) 1500.0))))
  (for (_array_element _array_index) (`self.WheelHits`)
    (bind (_bblockinghit _binitialoverlap _time _distance _location _impactpoint _normal _impactnormal _physmat _hitactor _hitcomponent _hitbonename _hititem _faceindex _tracestart) (`GameplayStatics.BreakHitResult` _array_element))
    (if _bblockinghit
      (bind (_output_position _output_stiffness _output_maxlength) (break `/Game/GGJPR2021/Blueprints/TractorBP/GGJ_TractorWheelSTR` (`|GetArrayItem` (`self.Wheels`) _array_index)))
      (`PrimitiveComponent.AddForceAtLocation` (`self.Cube`) (* _impactnormal (* (* (`PrimitiveComponent.GetMass` (`self.Cube`)) 1000.0) (- 1.0 (`KismetMathLibrary.FClamp` (/ _distance _output_maxlength))))) _tracestart "None")))
  (`PrimitiveComponent.AddForceAtLocationLocal` _cube_2 (`KismetMathLibrary.MakeVector` (* _throttle _returnvalue_x) (* _throttle _returnvalue_y)) (2.0 0.0 -2.0) "None")
  (if (>= _throttle 0.0)
    (`PrimitiveComponent.AddAngularImpulseInDegrees` _cube (`KismetMathLibrary.MakeVector` 0.0 0.0 _returnvalue) "None" true)
    (else
      (`PrimitiveComponent.AddAngularImpulseInDegrees` _cube (`KismetMathLibrary.MakeVector` 0.0 0.0 (* _returnvalue -1.0)) "None" true))))

(fn `CalcWheelHits`
  (bind _wheelhits (`self.WheelHits`))
  (bind _returnvalue (`SceneComponent.K2_GetComponentRotation` (`self.Cube`)))
  (`KismetArrayLibrary.Array_Clear` _wheelhits)
  (for (_array_element _array_index) (`self.Wheels`)
    (bind (_position _stiffness _maxlength) (break `/Game/GGJPR2021/Blueprints/TractorBP/GGJ_TractorWheelSTR` _array_element))
    (bind _returnvalue_2 (+ (`self.K2_GetActorLocation`) (`KismetMathLibrary.GreaterGreater_VectorRotator` _position _returnvalue)))
    (bind _outhit (`KismetSystemLibrary.LineTraceSingle` _returnvalue_2 (+ _returnvalue_2 (* (* (`KismetMathLibrary.GetUpVector` _returnvalue) _maxlength) -1.0)) "TraceTypeQuery1" false (`|MakeArray` self :!type "Actor Object Reference")))
    (`KismetArrayLibrary.Array_Set` _wheelhits _array_index _outhit true)))

(fn `DrawPhysicsDebug`
  (for (_array_element _array_index) (`self.WheelHits`)
    (bind (_bblockinghit _binitialoverlap _time _distance _location _impactpoint _normal _impactnormal _physmat _hitactor _hitcomponent _hitbonename _hititem _faceindex _tracestart _traceend) (`GameplayStatics.BreakHitResult` _array_element))
    (`KismetSystemLibrary.DrawDebugLine` _tracestart _traceend (struct :`R` 1.0 :`A` 1.0) 0.0 2.0)))

(fn `UserConstructionScript`)